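; BP_Camera is a security camera that sweeps, tracks the player and alerts a guard.
; A timeline sets a patrol rotation between positive and negative yaw, which Tick eases toward when no target exists.
; The view trigger makes Tick track the player along an inverted look vector, and writes Detected and AudioContactLocation to the blackboard of the BP_GuardEnemy found by GetActorOfClass.
; Leaving the trigger clears the target and Detected.
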(event `self.ReceiveBeginPlay`
  ;[1 1 1] Camera Passive Look
  (bind (_direction _camalpha) (`Timeline|CameraMovement`)
    (:`Update`
      (set `self.LastRotation` (`KismetMathLibrary.RLerp` (`KismetMathLibrary.MakeRotator` 0.0 (`self.CameraPitch`) (`self.CameraYaw`)) (`KismetMathLibrary.MakeRotator` 0.0 (`self.CameraPitch`) (* (`self.CameraYaw`) -1.0)) _camalpha)))))

(event `self.ReceiveTick`
  (params (DeltaSeconds :type "Float (single-precision)"))
  (bind _camera (`self.Camera`))
  ;[1 1 1] Camera Detection Follow
  (if (`self.HasTarget`)
    (`SceneComponent.K2_SetWorldRotation` (`self.Camera`) (`KismetMathLibrary.Conv_VectorToRotator` (`KismetMathLibrary.VInterpTo` (`KismetMathLibrary.Conv_RotatorToVector` (`SceneComponent.K2_GetComponentRotation` _camera)) (* (`KismetMathLibrary.GetDirectionUnitVector` (`SceneComponent.K2_GetComponentLocation` _camera) (`self.K2_GetActorLocation` (`self.TargetActor`))) (-1.0 -1.0 -1.0)) DeltaSeconds 5.0)) false false)
    (else
      (`SceneComponent.K2_SetRelativeRotation` (`self.Camera`) (`KismetMathLibrary.RInterpTo` (`SceneComponent.RelativeRotation` (`self.Camera`)) (`self.LastRotation`) DeltaSeconds 0.5) false false))))

(event `self.ViewTrigger.OnComponentBeginOverlap`
  (params (OverlappedComponent :type "PrimitiveComponent Object Reference") (OtherActor :type "Actor Object Reference") (OtherComp :type "PrimitiveComponent Object Reference") (OtherBodyIndex :type Integer) (bFromSweep :type Boolean) (SweepResult :type "HitResult Structure (by ref)"))
  (bind _asbp_player (cast `/Game/Blueprints/BP_Player` OtherActor))
  (set `self.TargetActor` _asbp_player)
  (set `self.HasTarget` true)
  (bind _returnvalue (`GameplayStatics.GetActorOfClass` "/Game/Blueprints/GuardCharacter/BP_GuardEnemy.BP_GuardEnemy_C"))
  (bind _asbp_guard_enemy (cast `/Game/Blueprints/GuardCharacter/BP_GuardEnemy` _returnvalue))
  (bind _returnvalue_2 (`AIBlueprintHelperLibrary.GetBlackboard` _asbp_guard_enemy))
  (`BlackboardComponent.SetValueAsVector` _returnvalue_2 "AudioContactLocation" (`self.K2_GetActorLocation` (`self.TargetActor`)))
  (`BlackboardComponent.SetValueAsBool` _returnvalue_2 "Detected" true))

(event `self.ViewTrigger.OnComponentEndOverlap`
  (params (OverlappedComponent :type "PrimitiveComponent Object Reference") (OtherActor :type "Actor Object Reference") (OtherComp :type "PrimitiveComponent Object Reference") (OtherBodyIndex :type Integer))
  (set `self.HasTarget` false)
  (set `self.TargetActor` null)
  (bind _returnvalue (`GameplayStatics.GetActorOfClass` "/Game/Blueprints/GuardCharacter/BP_GuardEnemy.BP_GuardEnemy_C"))
  (bind _asbp_guard_enemy (cast `/Game/Blueprints/GuardCharacter/BP_GuardEnemy` _returnvalue))
  (`BlackboardComponent.SetValueAsBool` (`AIBlueprintHelperLibrary.GetBlackboard` _asbp_guard_enemy) "Detected" false))

(fn `UserConstructionScript`)