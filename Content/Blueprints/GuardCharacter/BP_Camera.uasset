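; BP_Camera is a camera Blueprint in the GuardCharacter folder that performs a passive look rotation from BeginPlay.
; A timeline, CameraMovement, drives a rotator lerp on the Camera component's relative rotation.
; The yaw blends between CameraYaw and zero while pitch holds at CameraPitch and roll stays level.
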(event `self.ReceiveBeginPlay`
  ;[1 1 1] Camera Passive Look
  (bind (_direction _newtrack_0) (`Timeline|CameraMovement`)
    (:`Update`
      (`SceneComponent.K2_SetRelativeRotation` (`self.Camera`) (`KismetMathLibrary.RLerp` (`KismetMathLibrary.MakeRotator` 0.0 (`self.Camera Pitch`) (`self.Camera Yaw`)) (`KismetMathLibrary.MakeRotator` 0.0 (`self.Camera Pitch`) (* (`self.Camera Yaw`) 0.0)) _newtrack_0) false false))))

(fn `UserConstructionScript`)